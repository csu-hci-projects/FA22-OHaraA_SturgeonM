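; BP_CookingRegistry is a lookup table that maps item classes to what they cook into and how long cooking takes.
; GetResult and GetCookingTime each scan the CookingEntires array linearly for an entry whose IsA equals the searched class.
; A miss prints a red on-screen warning, then GetResult returns the input class unchanged and GetCookingTime returns a negative sentinel.
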(fn `GetCookingTime`
  (params (Search :type "Actor Class Reference"))
  (returns (CookingTime :type "Float (double-precision)"))
  (for _array_element (`self.CookingEntires`)
    (if (== (break `/Game/Blueprints/CookingEntry` _array_element) Search)
      (return (`.CookingTime_11_B133ABB14F6FB14A0416EAADAC468EA4` (break `/Game/Blueprints/CookingEntry` _array_element)))))
  (`KismetSystemLibrary.PrintString` (`KismetStringLibrary.Concat_StrStr` "COULD NOT FIND ITEM: " (`KismetSystemLibrary.GetClassDisplayName` Search)) true true (struct :`R` 1.0 :`B` 0.057999 :`A` 1.0))
  (return -1.0))

(fn `GetResult`
  (params (Search :type "Actor Class Reference"))
  (returns (Result :type "Actor Class Reference"))
  (for _array_element (`self.CookingEntires`)
    (if (== (break `/Game/Blueprints/CookingEntry` _array_element) Search)
      (return (`.CooksInto_5_FFDBA2FC4D6A4F31FEDD08B14671C3EC` (break `/Game/Blueprints/CookingEntry` _array_element)))))
  (`KismetSystemLibrary.PrintString` (`KismetStringLibrary.Concat_StrStr` "COULD NOT FIND ITEM: " (`KismetSystemLibrary.GetClassDisplayName` Search)) true true (struct :`R` 1.0 :`B` 0.057999 :`A` 1.0))
  (return Search))

(fn `UserConstructionScript`)