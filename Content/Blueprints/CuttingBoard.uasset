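; Cutting board actor that combines items placed on it into a new object, apparently for cooking.
; Its box overlaps maintain parallel arrays of actors and their classes, and each new overlap runs CombineItems through CheckCombinations.
; When every required class of a Combinations entry is present, it attempts to clear the board's contents and spawns the result at its location.
; An older map-based CombineMeal remains, but its calls never run.
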(event `self.Box.OnComponentBeginOverlap`
  (params (OverlappedComponent :type "PrimitiveComponent Object Reference") (OtherActor :type "Actor Object Reference") (OtherComp :type "PrimitiveComponent Object Reference") (OtherBodyIndex :type Integer) (bFromSweep :type Boolean) (SweepResult :type "HitResult Structure (by ref)"))
  (`KismetArrayLibrary.Array_Add` (`self.containedObjects_0`) (`GameplayStatics.GetObjectClass` OtherActor))
  (`KismetArrayLibrary.Array_Add` (`self.containedObjects`) OtherActor)
  (`self.CheckCombinations`)
  (`KismetSystemLibrary.PrintString` (`KismetSystemLibrary.GetDisplayName` OtherActor)))

(event `self.Box.OnComponentEndOverlap`
  (params (OverlappedComponent :type "PrimitiveComponent Object Reference") (OtherActor :type "Actor Object Reference") (OtherComp :type "PrimitiveComponent Object Reference") (OtherBodyIndex :type Integer))
  (bind _containedobjects (`self.containedObjects`))
  (bind _containedobjects_0 (`self.containedObjects_0`))
  (bind _returnvalue (`KismetArrayLibrary.Array_Find` _containedobjects OtherActor))
  (if (> _returnvalue -1)
    (`KismetArrayLibrary.Array_Remove` _containedobjects _returnvalue)
    (if (> (`KismetArrayLibrary.Array_Length` _containedobjects_0) _returnvalue)
      (`KismetArrayLibrary.Array_Remove` _containedobjects_0 _returnvalue))))

(fn `CheckCombinations`
  (`self.CombineItems`))

(fn `CombineItems`
  (locals (Found :type Boolean :default false) (Failed :type Boolean) (NewLocalVar_0 :type "Actor Class Reference") (NewLocalVar_1 :type "Actor Object Reference"))
  (bind _containedobjects_0 (`self.containedObjects_0`))
  (bind _containedobjects (`self.containedObjects`))
  ;[1 1 1] Foreach possible combination, check its requirements.
  (for _array_element (`self.Combinations`)
    (for _array_element_2 (`.Requires_5_3C1EA5DE402726F811CB1C865217686D` (break `/Game/Blueprints/Combination` _array_element))
      ;[1 1 1] Check the requirement with the things on the cutting board.  If any of them equal it, move on to the next requirement.  Otherwise, break with a failed flag.
      (if (not (`KismetArrayLibrary.Array_Contains` _containedobjects_0 _array_element_2))
        (set `local.Failed` true)
        (break)))
    ;[1 1 1] If at no point was the failed flag set, this must be a combinable thing, so replace all of the stuff with the ccombined object.
    (if (not (`local.Failed`))
      (bind _output_get (set `local.NewLocalVar_0` (break `/Game/Blueprints/Combination` _array_element)))
      (for (_array_element_3 _array_index) _containedobjects
        (bind _output_get_2 (set `local.NewLocalVar_1` _array_element_3))
        (`KismetArrayLibrary.Array_Remove` _containedobjects _array_index)
        (`self.K2_DestroyActor` _array_element_3)
        (`self.K2_DestroyActor` _output_get_2))
      (for (_ _array_index_2) _containedobjects_0
        (`KismetArrayLibrary.Array_Remove` _containedobjects_0 _array_index_2))
      (`|SpawnActorFromClass` _output_get (`KismetMathLibrary.Conv_VectorToTransform` (`self.K2_GetActorLocation`)) "Undefined" "OverrideRootScale" null null))))

(fn `combineMeal`
  (params (meal :type "Map of Actor Class Reference to Actor Object Reference (by ref)") (result :type "Actor Class Reference"))
  (locals (notValid :type Boolean))
  (for _array_element (`self.containedObjects`)
    (bind _returnvalue (`GameplayStatics.GetObjectClass` _array_element))
    (if (`.ReturnValue` (`BlueprintMapLibrary.Map_Find` meal _returnvalue))
      (`BlueprintMapLibrary.Map_Add` meal (`GameplayStatics.GetObjectClass` _array_element) _array_element)
      (else
        (`KismetSystemLibrary.PrintString` (`KismetSystemLibrary.GetClassDisplayName` _returnvalue)))))
  (bind _values (`BlueprintMapLibrary.Map_Values` meal))
  (for _array_element_2 _values
    (if (not (`KismetSystemLibrary.IsValid` _array_element_2))
      (set `local.notValid` true)))
  (if (not (`local.notValid`))
    (for _array_element_3 _values
      (`|VariableSetRef` (`BlueprintMapLibrary.Map_Find` meal (`GameplayStatics.GetObjectClass` _array_element_3)))
      (`self.K2_DestroyActor` _array_element_3))
    (`|SpawnActorFromClass` result (`KismetMathLibrary.Conv_VectorToTransform` (`self.K2_GetActorLocation`)) "Undefined" "OverrideRootScale" null null)))

(fn `UserConstructionScript`)