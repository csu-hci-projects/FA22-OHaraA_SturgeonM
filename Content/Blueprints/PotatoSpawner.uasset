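; Potato spawner actor that supplies a replacement whenever the last spawned potato leaves its box.
; On BeginPlay it spawns a BP_Potato at its own transform and stores it as LastPotato.
; When that tracked actor ends overlap with the Box, it spawns another and tracks the new one.
; AllowSpawn sets an AbleToSpawn flag, which the spawn logic does not check.
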(event `self.ReceiveBeginPlay`
  (bind _returnvalue (`|SpawnActorFromClass` "/Game/Blueprints/BP_Potato.BP_Potato_C" (`self.GetTransform`) "Undefined" "OverrideRootScale" null null))
  (set `self.lastPotato` _returnvalue))

(event `self.Box.OnComponentEndOverlap`
  (params (OverlappedComponent :type "PrimitiveComponent Object Reference") (OtherActor :type "Actor Object Reference") (OtherComp :type "PrimitiveComponent Object Reference") (OtherBodyIndex :type Integer))
  (if (== OtherActor (`self.lastPotato`))
    (bind _returnvalue (`|SpawnActorFromClass` "/Game/Blueprints/BP_Potato.BP_Potato_C" (`self.GetTransform`) "Undefined" "OverrideRootScale" null null))
    (set `self.lastPotato` _returnvalue)))

(event `self.Box.OnComponentBeginOverlap`
  (params (OverlappedComponent :type "PrimitiveComponent Object Reference") (OtherActor :type "Actor Object Reference") (OtherComp :type "PrimitiveComponent Object Reference") (OtherBodyIndex :type Integer) (bFromSweep :type Boolean) (SweepResult :type "HitResult Structure (by ref)")))

(fn `allowSpawn`
  (set `self.ableToSpawn` true))

(fn `UserConstructionScript`)