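; Oven actor that cooks the contents of a CookingWare placed in its overlap area.
; Begin and end overlap track the current cookware, and each tick calls its Cook while the oven is on and the OvenHatch is closed.
; Tick also toggles a smoke emitter, spawned inactive at BeginPlay, with the on state, and creates or destroys a fire sound as cooking starts or stops.
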(event `self.ReceiveBeginPlay`
  (bind _returnvalue (`GameplayStatics.SpawnEmitterAtLocation` "/Game/StarterContent/Particles/P_Smoke.P_Smoke" (`self.K2_GetActorLocation`) (struct) (`self.FireSize`) false "None" false))
  (set `self.Fire` _returnvalue))

(event `self.ReceiveActorBeginOverlap`
  (params (OtherActor :type "Actor Object Reference"))
  (bind _ascooking_ware (cast `/Game/Blueprints/CookingWare` OtherActor))
  (set `self.CookingWareCurrent` _ascooking_ware))

(event `self.ReceiveActorEndOverlap`
  (params (OtherActor :type "Actor Object Reference"))
  ;[1 1 1] Update current cooking ware, taken off
  (bind _ascooking_ware (cast `/Game/Blueprints/CookingWare` OtherActor))
  (if (== _ascooking_ware (`self.CookingWareCurrent`))
    (set `self.CookingWareCurrent` (`self.Nothing`))))

(event `self.ReceiveTick`
  (params (DeltaSeconds :type "Float (single-precision)"))
  ;[1 1 1] If  cooking ware is there, on tick, have the cooking ware cook whatever is on it.
  (`self.DealWithFire` (`self.IsOn`))
  (bind _confirmed (`self.CanCook`))
  (if _confirmed
    (`/Game/Blueprints/CookingWare.Cook` (`self.CookingWareCurrent`))
    (`/Engine/EditorBlueprintResources/StandardMacros.IsValid` (`self.FireSound`)
      (:`Is Not Valid`
        (bind _returnvalue (`GameplayStatics.SpawnSoundAtLocation` "/Game/VRTemplate/Audio/Fire01.Fire01" (`self.K2_GetActorLocation`) (struct) 1.0 1.0 0.0 null null))
        (set `self.FireSound` _returnvalue)))
    (else
      ;[1 1 1] Destroy fire sound
      (`/Engine/EditorBlueprintResources/StandardMacros.IsValid` (`self.FireSound`)
        (:`Is Valid`
          (`self.Destroy Current Fire Sound`))))))

(fn `CanCook`
  (returns (Confirmed :type Boolean))
  (bind _cookingwarecurrent (`self.CookingWareCurrent`))
  (`/Engine/EditorBlueprintResources/StandardMacros.IsValid` _cookingwarecurrent
    (:`Is Valid`
      (return (and (`self.IsOn`) (!= _cookingwarecurrent (`self.Nothing`)) (`/Game/Blueprints/OvenHatch.Closed` (`self.OvenHatch`)))))
    (:`Is Not Valid`
      (return false))))

(fn `DealWithFire`
  (params (`IsOn?` :type Boolean))
  (bind _fire (`self.Fire`))
  (if `IsOn?`
    (`/Engine/EditorBlueprintResources/StandardMacros.IsValid` _fire
      (:`Is Valid`
        (`ActorComponent.Activate` _fire false)))
    (else
      (`/Engine/EditorBlueprintResources/StandardMacros.IsValid` _fire
        (:`Is Valid`
          (`ActorComponent.Deactivate` _fire))))))

(fn `Destroy Current Fire Sound`
  (bind _firesound (`self.FireSound`))
  (`AudioComponent.SetPaused` _firesound true)
  (`ActorComponent.K2_DestroyComponent` _firesound))

(fn `UserConstructionScript`)