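; GeneralSpawner is a spawner actor that keeps replacing the object it spawns once that object leaves its area.
; On BeginPlay it spawns an actor of the Object class at its own transform and stores it as LastOne.
; When LastOne ends overlap with the Box component, Spawn runs again, producing the next one.
; AllowSpawn and the Box begin-overlap event are empty.
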(event `self.ReceiveBeginPlay`
  (`self.Spawn`))

(event `self.Box.OnComponentEndOverlap`
  (params (OverlappedComponent :type "PrimitiveComponent Object Reference") (OtherActor :type "Actor Object Reference") (OtherComp :type "PrimitiveComponent Object Reference") (OtherBodyIndex :type Integer))
  (if (== OtherActor (`self.lastOne`))
    (`self.Spawn`)))

(event `self.Box.OnComponentBeginOverlap`
  (params (OverlappedComponent :type "PrimitiveComponent Object Reference") (OtherActor :type "Actor Object Reference") (OtherComp :type "PrimitiveComponent Object Reference") (OtherBodyIndex :type Integer) (bFromSweep :type Boolean) (SweepResult :type "HitResult Structure (by ref)")))

(fn `allowSpawn`)

(fn `Spawn`
  (bind _returnvalue (`|SpawnActorFromClass` (`self.Object`) (`self.GetTransform`) "Undefined" "OverrideRootScale" null null))
  (set `self.lastOne` _returnvalue))

(fn `UserConstructionScript`)