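; TurnInPlate is a turn-in actor that scores meals delivered to it through overlap.
; On overlap, CheckIfMealComplete uses CheckStew to match the actor's exact class against BP_stew, currently the only recognized meal, for its score.
; The result goes to IncrementScore on the ScoreKepper found via GetActorOfClass.
; The overlapping actor is then destroyed, whether or not it matched.
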(event `self.ReceiveActorBeginOverlap`
  (params (OtherActor :type "Actor Object Reference"))
  (bind _score (`self.CheckIfMealComplete` OtherActor))
  (bind _returnvalue (`GameplayStatics.GetActorOfClass` "/Game/Blueprints/ScoreKepper.ScoreKepper_C"))
  (`/Game/Blueprints/ScoreKepper.IncrementScore` _returnvalue _score)
  (`self.K2_DestroyActor` OtherActor))

(fn `CheckIfMealComplete`
  (params (Overlap :type "Actor Object Reference"))
  (returns (Score :type Integer))
  (bind (_thismeal _score) (`self.CheckStew` Overlap))
  (if _thismeal
    (return _score)))

(fn `CheckStew`
  (params (Overlap :type "Actor Object Reference"))
  (returns (ThisMeal :type Boolean) (Score :type Integer))
  (return (== (`GameplayStatics.GetObjectClass` Overlap) "/Game/Blueprints/BP_stew.BP_stew_C") 1))

(fn `UserConstructionScript`)