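; A pressable stove button that toggles its linked Stove on and off.
; Each Tick it polls StoveButton's Touched state, sinking the mesh slightly while touched and restoring its start position on release.
; A WasTouching flag makes only the first frame of a touch flip IsOn, which is copied to the Stove and shown through Label.
; Two touch-edge helper functions are defined but not called here.
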(event `self.ReceiveBeginPlay`
  (set `self.StartPosition` (`SceneComponent.RelativeLocation` (`self.StaticMeshComponent1`))))

(event `self.ReceiveTick`
  (params (DeltaSeconds :type "Float (single-precision)"))
  (bind _output_get (set `self.Touching` (`/Game/Blueprints/StoveButton.touched` (`self.StoveButton`))))
  (if _output_get
    (`SceneComponent.K2_SetRelativeLocation` (`self.StaticMeshComponent1`) (+ (`self.StartPosition`) (0.0 0.0 -2.0)) false false)
    (if (not (`self.WasTouching`))
      (`self.SetNewOnValue`)
      (set `self.WasTouching` _output_get :!label _label)
      (`/Game/Blueprints/OnOffLabel.ChangeLabel` (`self.Label`) (`self.IsOn`)))
    (else
      (`SceneComponent.K2_SetRelativeLocation` (`self.StaticMeshComponent1`) (`self.StartPosition`) false false)
      (goto _label))))

(fn `SetNewOnValue`
  (bind _output_get (set `self.IsOn` (not (`self.IsOn`))))
  (set `/Game/Blueprints/BP_Stove.IsOn` _output_get (`self.Stove`)))

(fn `Touching Now Before Not`
  (returns (Value :type Boolean))
  (return (and (`self.Touching`) (not (`self.WasTouching`)))))

(fn `TouchingBeforeNowNot`
  (returns (Value :type Boolean))
  (return (and (not (`self.Touching`)) (`self.WasTouching`))))

(fn `UserConstructionScript`)