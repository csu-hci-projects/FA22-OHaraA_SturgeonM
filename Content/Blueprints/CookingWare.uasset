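; CookingWare is an actor Blueprint that tracks cooking progress for a piece of cookware.
; Initialize resets progress and stores a per-step increment, falling back to zero for non-positive values.
; Each Cook call adds that increment and fires the Done dispatcher once progress reaches or exceeds the completion threshold.
; It has no active Tick logic, so progress depends on external calls to Cook.
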(fn `Cook`
  (bind _output_get (set `self.Progress` (+ (`self.Progress`) (`self.Increment`))))
  (if (>= _output_get (`self.Completion`))
    (`self.Done`)))

(fn `Initialize`
  (params (Increment :type "Float (double-precision)"))
  (set `self.Progress` 0.0)
  (if (> Increment 0.0)
    (set `self.Increment` Increment)
    (else
      (set `self.Increment` 0.0))))

(fn `UserConstructionScript`)