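; Oven hatch actor that the player opens and closes by grabbing and pulling its handle.
; While held, Tick converts the handle's distance from its BeginPlay position into a clamped roll applied on top of the closed rotation.
; On release, the hatch snaps shut if nearly closed, and the handle returns to its anchor Scene component on the hatch.
; Tick also keeps a Closed flag updated by comparing rotation to the closed pose within a tolerance.
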(event `self.ReceiveBeginPlay`
  ;[1 1 1] Initialize the position of the handle and the closed position of the hatch
  (set `self.HandlePosition` (`SceneComponent.K2_GetComponentLocation` (`self.Handle`)))
  (set `self.RotationOrigin` (`self.K2_GetActorRotation`)))

(event `self.ReceiveTick`
  (params (DeltaSeconds :type "Float (single-precision)"))
  ;[1 1 1] Update whether or not hatch is closed.
  (set `self.Closed` (== (`self.K2_GetActorRotation`) (`self.RotationOrigin`) :`ErrorTolerance` 1.0))
  ;[1 1 1] Move hatch with handle while handle is held
  (if (`/Game/VRTemplate/Blueprints/GrabComponent.bIsHeld` (`self.GrabComponent`))
    (`self.K2_SetActorRotation` (`KismetMathLibrary.ComposeRotators` (`KismetMathLibrary.MakeRotator` (* (`KismetMathLibrary.FMin` (`KismetMathLibrary.FMax` (/ (`KismetMathLibrary.Vector_Distance` (`self.HandlePosition`) (`SceneComponent.K2_GetComponentLocation` (`self.Handle`))) (`self.MaxDistance`))) 0.9) -90.0)) (`self.RotationOrigin`)))))

(event `self.GrabComponent.OnDropped`
  (bind _rotationorigin (`self.RotationOrigin`))
  ;[1 1 1] Snap hatch to closed position if "close enough"
  (if (> (.roll (`self.K2_GetActorRotation`)) (- (.roll _rotationorigin) (`self.SnapCloseAllowance`)))
    (`self.K2_SetActorRotation` _rotationorigin))
  ;[1 1 1] Snap the handle to the correct position on the hatch
  (`SceneComponent.K2_SetWorldTransform` (`self.Handle`) (`SceneComponent.K2_GetComponentToWorld` (`self.Scene`)) false false))

(fn `UserConstructionScript`)