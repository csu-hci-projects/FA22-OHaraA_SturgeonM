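; Boss actor whose draining patience acts as a lose timer, triggering GameLost when it runs out.
; Each tick it turns its static mesh toward the player on yaw only by zeroing the look direction's Z, lowers patience scaled by delta time, and checks it against the end value.
; Appease adds patience back without capping it at the starting maximum.
; The current patience is printed every tick.
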(event `self.ReceiveBeginPlay`
  (set `self.PatienceLevel` (`self.PatienceMax`)))

(event `self.ReceiveTick`
  (params (DeltaSeconds :type "Float (single-precision)"))
  (`self.HandleLooking`)
  (`self.Decrement Patience`)
  (`self.CheckPatience`)
  (`KismetSystemLibrary.PrintString` (`KismetStringLibrary.Conv_DoubleToString` (`self.PatienceLevel`))))

(fn `Appease`
  (params (Amount :type "Float (double-precision)"))
  (set `self.PatienceLevel` (+ Amount (`self.PatienceLevel`))))

(fn `CheckPatience`
  (if (<= (`self.PatienceLevel`) (`self.PatienceEnd`))
    (`self.GameLost`)))

(fn `Decrement Patience`
  (set `self.PatienceLevel` (`KismetMathLibrary.FMax` (- (`self.PatienceLevel`) (* (* (`self.PatienceDecrementSpeed`) (`GameplayStatics.GetWorldDeltaSeconds`)) (`self.PatienceDecrement`))) (`self.PatienceEnd`))))

(fn `HandleLooking`
  (`SceneComponent.K2_SetWorldRotation` (`self.StaticMeshComponent`) (`KismetMathLibrary.Conv_VectorToRotator` (* (`KismetMathLibrary.Normal` (- (`self.K2_GetActorLocation` (`GameplayStatics.GetPlayerPawn` 0)) (`self.K2_GetActorLocation`))) (360.0 360.0 0.0))) false false))

(fn `UserConstructionScript`)